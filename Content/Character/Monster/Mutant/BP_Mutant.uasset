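; BP_Mutant is the Mutant monster, a melee AI character with high toughness and the grab-type flag enabled.
; On BeginPlay it runs the melee behavior tree on its AI controller, sets the AI state to Idle through the BB AI controller, then assigns its monster type, toughness and grab flag.
; The overlap, Tick and construction script graphs are empty.
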(event EventBeginPlay
  (bind _returnvalue (Class|BBAICharacter|GetBBAIController))
  (bind _self self)
  (bind _returnvalue_2 (AI|GetAIController _self))
  (Utilities|FlowControl|Sequence
    (:then_0
      (Utilities|IsValid _returnvalue_2
        (:Is%20Valid
          (AI|RunBehaviorTree _returnvalue_2 "/Game/Character/Monster/AI/MeleeAIBehaviorTree.MeleeAIBehaviorTree"))))
    (:then_1
      (Utilities|IsValid _returnvalue
        (:Is%20Valid
          (Class|BBAIController|ChangeAIState _returnvalue (Utilities|Enum|LiteralenumEMonsterState "EMS_Idle")))))
    (:then_2
      (Variables|Default|SetMonsterEnum "EM_Mutant")
      (Variables|Default|SetToughness "ET_High")
      (Variables|Default|SetCanGrabType true))))

(event Collision|EventActorBeginOverlap
  (params (OtherActor :type Actor%20Object%20Reference)))

(event EventTick
  (params (DeltaSeconds :type Float%20%28single-precision%29)))

(fn ConstructionScript)